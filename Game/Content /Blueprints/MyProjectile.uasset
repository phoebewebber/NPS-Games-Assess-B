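; Projectile Blueprint that deals point and small-radius damage on hit, destroys itself and plays surface-specific impact effects.
; The Hit event stores the impact point and hit component's rotation, then switches on the surface type from material slot 0's physical material.
; Per-surface custom events spawn particle emitters there and print debug strings.
; Unmatched surfaces reuse the sand effect, while the cave handler is empty.
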(event Custom|HitStone
  (bind _debrissize (Variables|Default|GetDebrisSize))
  (bind _impactlocation (Variables|Default|GetImpactLocation))
  (bind _impactactorrotation (Variables|Default|GetImpactActorRotation))
  ;[1 1 1] Stone
  (Utilities|FlowControl|Sequence
    (:then_1
      (Effects|SpawnEmitteratLocation "/Game/BallisticsVFX/Particles/Impacts/DynamicImpacts/Gravel/Gravel_Debris.Gravel_Debris" _impactlocation _impactactorrotation _debrissize))
    (:then_2
      (Effects|SpawnEmitteratLocation "/Game/BallisticsVFX/Particles/Impacts/DynamicImpacts/Gravel/Gravel_impact_2_Dyn.Gravel_impact_2_Dyn" _impactlocation _impactactorrotation _debrissize))
    (:then_3
      (Development|PrintString "Hit Gravel"))))

(event Custom|HitGrass
  ;[1 1 1] Grass
  (Utilities|FlowControl|Sequence
    (:then_1
      (Effects|SpawnEmitteratLocation "/Game/BallisticsVFX/Particles/Impacts/DynamicImpacts/Grass/Grass_impact_Dyn.Grass_impact_Dyn" (Variables|Default|GetImpactLocation) (Variables|Default|GetImpactActorRotation) "3.000000,3.000000,3.000000"))
    (:then_2
      (Development|PrintString "Hit Grass/Bush"))))

(event Custom|HitWater
  ;[1 1 1] Water
  (Utilities|FlowControl|Sequence
    (:then_1
      (Effects|SpawnEmitteratLocation "/Game/BallisticsVFX/Particles/Impacts/DynamicImpacts/Water/Water_impact_Dyn.Water_impact_Dyn" (Variables|Default|GetImpactLocation) (Variables|Default|GetImpactActorRotation) (Variables|Default|GetDebrisSize)))
    (:then_2
      (Development|PrintString "Hit Wood"))))

(event Custom|HitSand
  (bind _impactlocation (Variables|Default|GetImpactLocation))
  (bind _impactactorrotation (Variables|Default|GetImpactActorRotation))
  (bind _debrissize (Variables|Default|GetDebrisSize))
  ;[1 1 1] Sand/Default
  (Utilities|FlowControl|Sequence
    (:then_2
      (Effects|SpawnEmitteratLocation "/Game/BallisticsVFX/Particles/Impacts/DynamicImpacts/Sand/Sand_Debris.Sand_Debris" _impactlocation _impactactorrotation _debrissize))
    (:then_3
      (Effects|SpawnEmitteratLocation "/Game/BallisticsVFX/Particles/Impacts/DynamicImpacts/Sand/Sand_impact_2_Dyn.Sand_impact_2_Dyn" _impactlocation _impactactorrotation _debrissize))
    (:then_4
      (Development|PrintString "Hit Desert"))))

(event Custom|HitMetal
  (bind _debrissize (Variables|Default|GetDebrisSize))
  (bind _impactlocation (Variables|Default|GetImpactLocation))
  (bind _impactactorrotation (Variables|Default|GetImpactActorRotation))
  ;[1 1 1] Metal
  (Utilities|FlowControl|Sequence
    (:then_1
      (Effects|SpawnEmitteratLocation "/Game/BallisticsVFX/Particles/Impacts/DynamicImpacts/Metal/Metal_Debris.Metal_Debris" _impactlocation _impactactorrotation _debrissize))
    (:then_2
      (Effects|SpawnEmitteratLocation "/Game/BallisticsVFX/Particles/Impacts/DynamicImpacts/Metal/Metal_impact_Dyn2.Metal_impact_Dyn2" _impactlocation _impactactorrotation _debrissize))
    (:then_3
      (Development|PrintString "Hit Metal"))))

(event Custom|HitWood
  ;[1 1 1] Wood
  (Utilities|FlowControl|Sequence
    (:then_1
      (Effects|SpawnEmitteratLocation "/Game/BallisticsVFX/Particles/Impacts/DynamicImpacts/Wood/Wood_impact_Dyn.Wood_impact_Dyn" (Variables|Default|GetImpactLocation) (Variables|Default|GetImpactActorRotation) (Variables|Default|GetDebrisSize)))
    (:then_2
      (Development|PrintString "Hit Wood"))))

(event Custom|HitFlesh
  ;[1 1 1] Blood
  (Utilities|FlowControl|Sequence
    (:then_1
      (Effects|SpawnEmitteratLocation "/Game/BallisticsVFX/Particles/Impacts/DynamicImpacts/Flesh/Blood_cloud_Dyn.Blood_cloud_Dyn" (Variables|Default|GetImpactLocation) (Variables|Default|GetImpactActorRotation) (Variables|Default|GetDebrisSize)))
    (:then_2
      (Development|PrintString "Hit Flesh"))))

(event Custom|HitDefault
  (bind _impactlocation (Variables|Default|GetImpactLocation))
  (bind _impactactorrotation (Variables|Default|GetImpactActorRotation))
  (bind _debrissize (Variables|Default|GetDebrisSize))
  ;[1 1 1] Sand/Default
  (Utilities|FlowControl|Sequence
    (:then_2
      (Effects|SpawnEmitteratLocation "/Game/BallisticsVFX/Particles/Impacts/DynamicImpacts/Sand/Sand_Debris.Sand_Debris" _impactlocation _impactactorrotation _debrissize))
    (:then_3
      (Effects|SpawnEmitteratLocation "/Game/BallisticsVFX/Particles/Impacts/DynamicImpacts/Sand/Sand_impact_2_Dyn.Sand_impact_2_Dyn" _impactlocation _impactactorrotation _debrissize))
    (:then_4
      (Development|PrintString "Hit Desert"))))

(event Custom|HitCave
  ;[1 1 1] Cave
)

(event Collision|EventHit
  (params (MyComp :type Primitive%20Component%20Object%20Reference) (Other :type Actor%20Object%20Reference) (OtherComp :type Primitive%20Component%20Object%20Reference) (bSelfMoved :type Boolean) (HitLocation :type Vector :default "0, 0, 0") (HitNormal :type Vector :default "0, 0, 0") (NormalImpulse :type Vector :default "0, 0, 0") (Hit :type Hit%20Result%20Structure%20%28by%20ref%29))
  (bind (_bblockinghit _binitialoverlap _time _distance _location _impactpoint _normal _impactnormal _physmat _hitactor _hitcomponent) (Collision|BreakHitResult Hit))
  (Variables|Default|SetImpactLocation _impactpoint)
  (Variables|Default|SetImpactActorRotation (Transformation|GetWorldRotation _hitcomponent))
  (Game|Damage|ApplyDamage Other 25.0 0 0)
  (Game|Damage|ApplyRadialDamage 5e+01 _impactpoint 2e+01 0 0 0 0 false "ECC_Visibility")
  (Utilities|FlowControl|Sequence
    (:then_0
      (Actor|DestroyActor) ; Then destroy this projectile
    )
    (:then_1
      ;[1 1 1] Get Surface and Cast to custom event
      (switch Utilities|FlowControl|Switch|SwitchonEPhysicalSurface (Variables|/Script/Engine.PhysicalMaterial|GetSurfaceType (Class|MaterialInterface|GetPhysicalMaterial (Rendering|Material|GetMaterial _hitcomponent 0)))
        (:SurfaceType_Default
          (CallFunction|HitDefault))
        (:SurfaceType1
          (CallFunction|HitSand))
        (:SurfaceType2
          (CallFunction|HitCave))
        (:SurfaceType6
          (CallFunction|HitStone))
        (:SurfaceType7
          (CallFunction|HitMetal))
        (:SurfaceType9
          (CallFunction|HitWood))
        (:SurfaceType10
          (CallFunction|HitGrass))
        (:SurfaceType11
          (CallFunction|HitFlesh))
        (:SurfaceType12
          (CallFunction|HitWater))))))

(fn ConstructionScript)