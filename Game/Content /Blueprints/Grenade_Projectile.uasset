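; Grenade launcher projectile that deals heavy damage to the actor it hits plus radial damage around the impact point, then destroys itself.
; The Hit event drives everything, spawning two sand decals and two explosion emitters at the impact after the destroy call, along with a "Hit Desert" debug print.
; Impact effects are always sand, as the physical material surface lookup is left unconnected.
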(event Collision|EventHit
  (params (MyComp :type Primitive%20Component%20Object%20Reference) (Other :type Actor%20Object%20Reference) (OtherComp :type Primitive%20Component%20Object%20Reference) (bSelfMoved :type Boolean) (HitLocation :type Vector :default "0, 0, 0") (HitNormal :type Vector :default "0, 0, 0") (NormalImpulse :type Vector :default "0, 0, 0") (Hit :type Hit%20Result%20Structure%20%28by%20ref%29))
  (bind (_bblockinghit _binitialoverlap _time _distance _location _impactpoint _normal _impactnormal _physmat _hitactor _hitcomponent _hitbonename) (Collision|BreakHitResult Hit))
  (bind _decalsize (Variables|Default|GetDecalSize))
  (bind _debrissize (Variables|Default|GetDebrisSize))
  (Variables|Default|SetImpactLocation _impactpoint)
  (Variables|Default|SetImpactActorRotation (Transformation|GetWorldRotation _hitcomponent))
  (Game|Damage|ApplyDamage Other 2.2e+03 0 0)
  (Game|Damage|ApplyRadialDamage 4e+02 _impactpoint 1.5e+02 0 0 0 0 false "ECC_Visibility")
  (Utilities|FlowControl|Sequence
    (:then_0
      (Actor|DestroyActor) ; Then destroy this projectile
    )
    (:then_1
      ;[1 1 1] Sand/Default
      (Utilities|FlowControl|Sequence
        (:then_0
          (Class|GameplayStatics|SpawnDecalAttached "/Game/BallisticsVFX/Decals/Decals_Sand.Decals_Sand" _decalsize _hitcomponent _hitbonename _impactpoint "0, 0, 0" "KeepRelativeOffset" (Variables|Default|GetDecal%20Life%20Span)))
        (:then_1
          (Rendering|Decal|SpawnDecalatLocation "/Game/BallisticsVFX/Decals/Splashers/Decal_SandSplatter.Decal_SandSplatter" _decalsize (Variables|Default|GetImpactLocation) (Variables|Default|GetImpactActorRotation) 0.0))
        (:then_2
          (Effects|SpawnEmitteratLocation "/Game/BallisticsVFX/Particles/Explosive/Explosion_GrenadeLauncher_1.Explosion_GrenadeLauncher_1" (Variables|Default|GetImpactLocation) (Variables|Default|GetImpactActorRotation) _debrissize))
        (:then_3
          (Effects|SpawnEmitteratLocation "/Game/Effects/Effects/VehicleEffects/P_Explosion.P_Explosion" (Variables|Default|GetImpactLocation) (Variables|Default|GetImpactActorRotation) _debrissize))
        (:then_4
          (Development|PrintString "Hit Desert"))))))

(fn ConstructionScript)