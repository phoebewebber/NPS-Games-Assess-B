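; BP_Candelabra is a configurable three-armed candelabra prop with left, center and right candle slots.
; The Construction Script uses per-slot booleans to add a static mesh component at each candle's fixed transform.
; A nested lit flag adds a second mesh at the same transform, so a candle can only be lit when present.
; The event graph holds only disabled default events, so there is no runtime logic.
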(event EventBeginPlay)

(event EventActorBeginOverlap
  (params (OtherActor :type Actor%20Object%20Reference)))

(event EventTick
  (params (DeltaSeconds :type Float%20%28single-precision%29)))

(fn ConstructionScript
  (Utilities|FlowControl|Sequence
    (:then_0
      (if (Variables|Default|GetbAddLeftCandel)
        (AddComponent|AddStaticMeshComponent false (Math|Transform|MakeTransform "0.000000,18.666748,35.899994"))
        (if (Variables|Default|GetbLeftCandelShouldBeLit)
          (AddComponent|AddStaticMeshComponent false (Math|Transform|MakeTransform "0.000000,18.666748,35.899994")))))
    (:then_1
      (if (Variables|Default|GetbAddCenterCandel)
        (AddComponent|AddStaticMeshComponent false (Math|Transform|MakeTransform "0, 0,42.000000" "0,90.000000, 0"))
        (if (Variables|Default|GetbCenterCandelShouldBeLit)
          (AddComponent|AddStaticMeshComponent false (Math|Transform|MakeTransform "0, 0,42.000000" "0,90.000000, 0")))))
    (:then_2
      (if (Variables|Default|GetbAddRightCandel)
        (AddComponent|AddStaticMeshComponent false (Math|Transform|MakeTransform "0.000000,-18.666748,35.899994" "0,180.000000, 0"))
        (if (Variables|Default|GetbRightCandelShouldBeLit)
          (AddComponent|AddStaticMeshComponent false (Math|Transform|MakeTransform "0.000000,-18.666748,35.899994" "0,180.000000, 0")))))))